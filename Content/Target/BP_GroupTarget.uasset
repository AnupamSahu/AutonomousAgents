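; BP_GroupTarget is a moving target actor that loops continuously around the world origin.
; Every Tick, MoveRadial sets its absolute location from sine and cosine of game time, with X and Z sharing the cosine to form a tilted elliptical path.
; An alternative MoveLinearPingPong function oscillates it along the Y axis using accumulated delta time, but its call never runs.
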(event `self.ReceiveTick`
  (params (DeltaSeconds :type "Float (single-precision)"))
  (`self.MoveRadial` 500.0 100.0))

(fn `MoveLinearPingPong`
  (params (DeltaTime :type "Float (double-precision)"))
  (bind _output_get (set `self.Time` (+ DeltaTime (`self.Time`))))
  (`self.K2_SetActorLocation` (`KismetMathLibrary.MakeVector` 0.0 (* (`KismetMathLibrary.DegSin` (* _output_get 100.0)) (`KismetMathLibrary.FClamp` 1000.0 -10000.0 10000.0)))))

(fn `MoveRadial`
  (params (Radius :type "Float (double-precision)" :default 1000.0) (Speed :type "Float (double-precision)" :default 10.0))
  (bind _returnvalue (* Speed (`KismetSystemLibrary.GetGameTimeInSeconds`)))
  (bind _returnvalue_2 (* Radius (`KismetMathLibrary.DegCos` _returnvalue)))
  (`self.K2_SetActorLocation` (`KismetMathLibrary.MakeVector` _returnvalue_2 (* Radius (`KismetMathLibrary.DegSin` _returnvalue)) _returnvalue_2)))

(fn `UserConstructionScript`)